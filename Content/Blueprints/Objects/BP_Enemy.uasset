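; Enemy actor Blueprint that takes typed damage and dies when its health runs out.
; On BeginPlay it caches the DamageValues map from BP_ThirdPersonGameMode.
; Its Damage event, while Alive, subtracts the value looked up for the given type, then clears Alive at zero or below.
; Remaining HP and the kill are reported only through Print String messages.
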(event `self.ReceiveBeginPlay`
  (bind _asbp_third_person_game_mode (cast `/Game/ThirdPerson/Blueprints/BP_ThirdPersonGameMode` (`GameplayStatics.GetGameMode`)))
  (set `self.DamageValues` (`/Game/ThirdPerson/Blueprints/BP_ThirdPersonGameMode.DamageValues` _asbp_third_person_game_mode)))

(event `/Game/Blueprints/Interfaces/BPI_Damage.Damage`
  (params (Type :type String))
  (if (`self.bAlive`)
    (set `self.Health` (- (`self.Health`) (`BlueprintMapLibrary.Map_Find` (`self.DamageValues`) Type)))
    (if (<= (`self.Health`) 0)
      (set `self.bAlive` false)
      (`KismetSystemLibrary.PrintString` "Enemy Killed")
      (else
        (`KismetSystemLibrary.PrintString` (`KismetStringLibrary.Concat_StrStr` (`KismetStringLibrary.Conv_IntToString` (`self.Health`)) "HP Left"))))))

(fn `UserConstructionScript`)