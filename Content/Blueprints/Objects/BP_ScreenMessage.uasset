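; BP_ScreenMessage is an interactable or pop-up actor that shows a text message on screen.
; Each interaction while active toggles pausing, swaps the HUD for the message widget, and optionally switches the view to its own camera; pop-up or one-time instances self-destroy on closing.
; Pop-ups trigger on character overlap, and a bound key-obtained event can deactivate it.
; The camera's CRT post-process filter follows the options menu checkbox.
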(event `self.ReceiveBeginPlay`
  (`|ExecutionSequence`
    (:`then_0`
      ; Wait for Hud on Viewport
      (`KismetSystemLibrary.Delay` 0.2)
      (bind _foundwidgets (`WidgetBlueprintLibrary.GetAllWidgetsOfClass` "/Game/Blueprints/UI/WBP_Hud.WBP_Hud_C"))
      (for _array_element _foundwidgets
        (`/Engine/EditorBlueprintResources/StandardMacros.IsValid` _array_element
          (:`Is Valid`
            (set `self.HudReference` _array_element)
            (break))))
      (bind _returnvalue (`|CreateWidget` "/Game/Blueprints/UI/WBP_Message.WBP_Message_C"))
      (set `self.WidgetReference` _returnvalue)
      (bind _asgi_instance (cast `/Game/Blueprints/GameInstance/GI_Instance` (`GameplayStatics.GetGameInstance`)))
      (bind _optionsmenu (`/Game/Blueprints/GameInstance/GI_Instance.OptionsMenu` _asgi_instance))
      (add `/Game/Blueprints/UI/Menu/BP_Options.FilterEvent` _optionsmenu (delegate `Enable/DisableCRT`))
      (`self.Enable/DisableCRT` (`CheckBox.IsChecked` (`/Game/Blueprints/UI/Menu/BP_Options.CheckBox_Filter` _optionsmenu))))
    (:`then_1`
      (`KismetSystemLibrary.Delay` 0.2)
      (set `/Game/Blueprints/UI/WBP_Message.TextMessage` (`self.Message`) (`self.WidgetReference`)))))

(event `Enable/DisableCRT`
  (params (Checked :type Boolean))
  (bind _array (break `WeightedBlendables` (`.WeightedBlendables` (break `PostProcessSettings` (`CameraComponent.PostProcessSettings` (`self.Camera`))))))
  (if Checked
    (if (`KismetArrayLibrary.Array_IsEmpty` _array)
      (`KismetArrayLibrary.Array_Add` _array (make `WeightedBlendable` 1.0 (`self.Filter`))))
    (else
      (`KismetArrayLibrary.Array_Remove` _array))))

(event `/Game/Blueprints/Interfaces/BPI_Interact.Interact`
  (if (`self.bActive?`)
    (if (`self.bCameraChange?`)
      (`self.CameraChange`))
    (`/Engine/EditorBlueprintResources/StandardMacros.FlipFlop`
      (:`A`
        (`GameplayStatics.SetGamePaused` true)
        (`Widget.RemoveFromParent` (`self.HudReference`))
        (`UserWidget.AddToViewport` (`self.WidgetReference`) 0))
      (:`B`
        (`GameplayStatics.SetGamePaused` false)
        (`Widget.RemoveFromParent` (`self.WidgetReference`))
        (`UserWidget.AddToViewport` (`self.HudReference`) 0)
        (if (or (`self.bPopUp`) (`self.bOneTime`))
          (`self.K2_DestroyActor`))))))

(event `CameraChange`
  (bind _returnvalue (`PlayerState.GetPlayerController` (`Pawn.PlayerState` (`GameplayStatics.GetPlayerPawn` 0))))
  (`/Engine/EditorBlueprintResources/StandardMacros.FlipFlop`
    (:`A`
      (set `self.LastCamera` (`Controller.GetViewTarget` _returnvalue))
      (`PlayerController.SetViewTargetWithBlend` _returnvalue self 0.0 "VTBlend_Linear" 0.0 false))
    (:`B`
      (`PlayerController.SetViewTargetWithBlend` _returnvalue (`self.LastCamera`) 0.0 "VTBlend_Linear" 0.0 false))))

(event `GetKeyEvent`
  (add `/Game/Blueprints/Objects/BP_Key.KeyObtained` (`self.Key`) (delegate `Deactivate`)))

(event `Deactivate`
  (set `self.bActive?` false))

(event `self.Box.OnComponentBeginOverlap`
  (params (OverlappedComponent :type "PrimitiveComponent Object Reference") (OtherActor :type "Actor Object Reference") (OtherComp :type "PrimitiveComponent Object Reference") (OtherBodyIndex :type Integer) (bFromSweep :type Boolean) (SweepResult :type "HitResult Structure (by ref)"))
  (if (`self.bPopUp`)
    (bind _asbp_character (cast `/Game/Blueprints/Characters/BP_Character` OtherActor))
    (`/Engine/EditorBlueprintResources/StandardMacros.IsValid` _asbp_character
      (:`Is Valid`
        (`/Game/Blueprints/Interfaces/BPI_Interact.Interact`)))))

(fn `UserConstructionScript`
  (`parent.UserConstructionScript`))