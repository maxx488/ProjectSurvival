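; BP_Key is a key pickup that the player collects by interacting with it.
; On BeginPlay it creates a dynamic material instance on its static mesh and tints it with its MaterialColor value.
; Its Interact event runs the parent logic, fires the KeyObtained dispatcher for any bound listeners, plays a 2D pickup sound and destroys the actor.
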(event `self.ReceiveBeginPlay`
  (`parent.ReceiveBeginPlay`)
  (bind _returnvalue (`PrimitiveComponent.CreateDynamicMaterialInstance` (`self.StaticMesh`) 0 (`PrimitiveComponent.GetMaterial` (`self.StaticMesh`) 0) "None"))
  (bind _output_get (set `self.MaterialInstance` _returnvalue))
  (`MaterialInstanceDynamic.SetVectorParameterValue` _output_get "Color" (`self.MaterialColor`)))

(event `/Game/Blueprints/Interfaces/BPI_Interact.Interact`
  (`parent.Interact`)
  (`self.KeyObtained`)
  (`GameplayStatics.PlaySound2D` "/Game/Sounds/TakeItem.TakeItem" 1.0 1.0 0.0 null null false)
  (`self.K2_DestroyActor`))

(fn `UserConstructionScript`
  (`parent.UserConstructionScript`))