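; BP_Weapon is an interactable weapon pickup that gives its weapon Type to the player character.
; On Interact it runs the parent logic, then adds Type to BP_Character's WeaponSlots map, using the current key count as the new slot index.
; That slot and Type become the active slot and weapon, then the pickup destroys itself and calls WeaponPickEvent.
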(event `self.Interact`
  (`parent.Interact`)
  (bind _asbp_character (cast `/Game/Blueprints/Characters/BP_Character` (`GameplayStatics.GetPlayerCharacter` 0)))
  (bind _weaponslots (`/Game/Blueprints/Characters/BP_Character.WeaponSlots` _asbp_character))
  (bind _keys (`BlueprintMapLibrary.Map_Keys` _weaponslots))
  (bind _returnvalue (`KismetArrayLibrary.Array_Length` _keys))
  (set `/Game/Blueprints/Characters/BP_Character.ActiveSlot` _returnvalue _asbp_character)
  (`BlueprintMapLibrary.Map_Add` _weaponslots _returnvalue (`self.Type`))
  (set `/Game/Blueprints/Characters/BP_Character.ActiveWeapon` (`self.Type`) _asbp_character)
  (`self.K2_DestroyActor`)
  (`self.WeaponPickEvent`))

(fn `UserConstructionScript`
  (`parent.UserConstructionScript`))