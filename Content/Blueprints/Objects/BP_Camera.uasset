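; BP_Camera is a camera that toggles a CRT post-process filter according to the options menu.
; Shortly after BeginPlay it gets the options menu from GI_Instance, binds to its filter event and applies the current checkbox state.
; The toggle adds the filter material as a weighted blendable when the camera's post-process array is empty, and removes the first entry when unchecked.
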(event `self.ReceiveBeginPlay`
  (`KismetSystemLibrary.Delay` 0.2)
  (bind _asgi_instance (cast `/Game/Blueprints/GameInstance/GI_Instance` (`GameplayStatics.GetGameInstance`)))
  (bind _optionsmenu (`/Game/Blueprints/GameInstance/GI_Instance.OptionsMenu` _asgi_instance))
  (add `/Game/Blueprints/UI/Menu/BP_Options.FilterEvent` _optionsmenu (delegate `Enable/DisableCRT`))
  (`self.Enable/DisableCRT` (`CheckBox.IsChecked` (`/Game/Blueprints/UI/Menu/BP_Options.CheckBox_Filter` _optionsmenu))))

(event `Enable/DisableCRT`
  (params (Checked :type Boolean))
  (bind _array (break `WeightedBlendables` (`.WeightedBlendables` (break `PostProcessSettings` (`CameraComponent.PostProcessSettings` (`self.CameraComponent`))))))
  (if Checked
    (if (`KismetArrayLibrary.Array_IsEmpty` _array)
      (`KismetArrayLibrary.Array_Add` _array (make `WeightedBlendable` 1.0 (`self.Filter`))))
    (else
      (`KismetArrayLibrary.Array_Remove` _array))))

(fn `UserConstructionScript`)