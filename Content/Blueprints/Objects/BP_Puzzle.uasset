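; BP_Puzzle is an interactable lock that raises a referenced Gate once its Key has been obtained.
; GetKeyEvent binds Unlock to the Key's KeyObtained event, which sets Solved.
; When solved, Interact plays the GateUp timeline, lerping the gate's current Z toward a fixed height above its position at interaction.
; The puzzle actor destroys itself when the timeline finishes.
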(event `/Game/Blueprints/Interfaces/BPI_Interact.Interact`
  (bind _gate (`self.Gate`))
  (bind (_returnvalue_x _returnvalue_y _returnvalue_z) (`KismetMathLibrary.BreakVector` (`self.K2_GetActorLocation` (`self.Gate`))))
  (bind (_returnvalue_x_2 _returnvalue_y_2 _returnvalue_z_2) (`KismetMathLibrary.BreakVector` (`self.K2_GetActorLocation` _gate)))
  (if (`self.Solved`)
    (set `self.ZLocation` _returnvalue_z)
    (bind (_direction _elevate) (`Timeline|GateUp` :!via `PlayFromStart`)
      (:`Update`
        (`self.K2_SetActorLocation` _gate (`KismetMathLibrary.MakeVector` _returnvalue_x_2 _returnvalue_y_2 (`KismetMathLibrary.Lerp` _returnvalue_z_2 (+ (`self.ZLocation`) 250.0) _elevate)) false false))
      (:`Finished`
        (`self.K2_DestroyActor`)))))

(event `GetKeyEvent`
  (add `/Game/Blueprints/Objects/BP_Key.KeyObtained` (`self.Key`) (delegate `Unlock`)))

(event `Unlock`
  (set `self.Solved` true))

(fn `UserConstructionScript`)