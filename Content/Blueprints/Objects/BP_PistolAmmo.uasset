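; BP_PistolAmmo is an interactable ammo pickup, named for pistol ammo, that replenishes the player's ammo.
; On Interact, it casts player 0's character to BP_Character and adds its Ammo amount to the AmmoCount map entry keyed by its Type.
; It passes the new total as a string to CallAmmoUpdate just before writing the map, then destroys itself.
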(event `/Game/Blueprints/Interfaces/BPI_Interact.Interact`
  (bind _asbp_character (cast `/Game/ThirdPerson/Blueprints/BP_Character` (`GameplayStatics.GetPlayerCharacter` 0)))
  (bind _returnvalue (+ (`BlueprintMapLibrary.Map_Find` (`/Game/ThirdPerson/Blueprints/BP_Character.AmmoCount` _asbp_character) (`self.Type`)) (`self.Ammo`)))
  (`/Game/ThirdPerson/Blueprints/BP_Character.AmmoUpdate` _asbp_character (`KismetStringLibrary.Conv_IntToString` _returnvalue))
  (`BlueprintMapLibrary.Map_Add` (`/Game/ThirdPerson/Blueprints/BP_Character.AmmoCount` _asbp_character) (`self.Type`) _returnvalue)
  (`self.K2_DestroyActor`))

(fn `UserConstructionScript`
  (`parent.UserConstructionScript`))