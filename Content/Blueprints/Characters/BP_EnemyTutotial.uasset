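; Tutorial enemy character that starts inert and turns into an active zombie after a weapon pickup event.
; On BeginPlay it creates a dynamic mesh material, gives its AI controller a very short life span and disables movement.
; WeaponPick binds Awake to the weapon's pick event; Awake runs the Zombify timeline to blend the zombie material parameter.
; When the timeline finishes, a new AIC_EnemyController possesses it and walking resumes.
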(event `self.ReceiveBeginPlay`
  (bind _skeletalmesh (`self.SkeletalMesh`))
  (`parent.ReceiveBeginPlay`)
  (bind _returnvalue (`PrimitiveComponent.CreateDynamicMaterialInstance` _skeletalmesh 0 (`PrimitiveComponent.GetMaterial` _skeletalmesh 0) "None"))
  (set `self.MaterialInstance` _returnvalue)
  ; Reemplazar por comportamiento
  (`self.SetLifeSpan` (`AIBlueprintHelperLibrary.GetAIController` self) 0.1)
  (`CharacterMovementComponent.DisableMovement` (`self.CharacterMovement`)))

(event `WeaponPick`
  (add `/Game/Blueprints/Objects/BP_Weapon.WeaponPickEvent` (`self.WeaponPicked`) (delegate `Awake`)))

(event `Awake`
  (bind (_direction _zombiealpha) (`Timeline|Zombify` :!via `PlayFromStart`)
    (:`Update`
      (`MaterialInstanceDynamic.SetScalarParameterValue` (`self.MaterialInstance`) "bZombie?" (`KismetMathLibrary.Lerp` 0.0 1.0 _zombiealpha)))
    (:`Finished`
      (bind _returnvalue (`|SpawnActorFromClass` "/Game/Blueprints/Controllers/AIC_EnemyController.AIC_EnemyController_C" (`KismetMathLibrary.MakeTransform` (0.0 0.0 0.0)) "Undefined" "MultiplyWithRoot" null null))
      (`Controller.Possess` _returnvalue self)
      (`CharacterMovementComponent.SetMovementMode` (`self.CharacterMovement`) "MOVE_Walking" 0))))

(fn `UserConstructionScript`
  (`parent.UserConstructionScript`))