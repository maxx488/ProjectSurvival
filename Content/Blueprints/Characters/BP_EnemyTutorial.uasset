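; Tutorial enemy that starts as an immobile guard playing a pain loop, with its AI controller quickly expired.
; WeaponPick binds Awake to the weapon-picked event; Awake stands the guard up and plays the tutorial level sequence with player input and HUD off.
; A timed timeline then fades a dynamic material into its zombie look.
; Afterwards it gains a new AI controller, walking movement and zombie AnimBP, and player control and HUD return.
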(event `self.ReceiveBeginPlay`
  (bind _skeletalmesh (`self.SkeletalMesh`))
  (`parent.ReceiveBeginPlay`)
  (bind _returnvalue (`PrimitiveComponent.CreateDynamicMaterialInstance` _skeletalmesh 0 (`PrimitiveComponent.GetMaterial` _skeletalmesh 0) "None"))
  (set `self.MaterialInstance` _returnvalue)
  ; Reemplazar por comportamiento
  (`self.SetLifeSpan` (`AIBlueprintHelperLibrary.GetAIController` self) 0.1)
  (`CharacterMovementComponent.DisableMovement` (`self.CharacterMovement`))
  (`SkeletalMeshComponent.PlayAnimation` (`self.Mesh`) "/Game/Animations/A_GuardPain.A_GuardPain" true))

(event `WeaponPick`
  (add `/Game/Blueprints/Objects/BP_Weapon.WeaponPickEvent` (`self.WeaponPicked`) (delegate `Awake`)))

(event `Awake`
  (bind _playerref (`self.PlayerRef`))
  (bind _playerref_2 (`self.PlayerRef`))
  (`KismetSystemLibrary.Delay` 0.2)
  (`SkeletalMeshComponent.PlayAnimation` (`self.Mesh`) "/Game/Animations/A_GuardStandUp.A_GuardStandUp" false)
  (`self.DisableInput` _playerref (`GameplayStatics.GetPlayerController` 0))
  (`Widget.RemoveFromParent` (`/Game/Blueprints/Characters/BP_Character.Hud` _playerref))
  (bind (_outactor _returnvalue) (`LevelSequencePlayer.CreateLevelSequencePlayer` "/Game/Blueprints/Cinematics/LS_Tutorial.LS_Tutorial"))
  (`MovieSceneSequencePlayer.Play` _returnvalue)
  (`KismetSystemLibrary.Delay` 15.0)
  (bind (_direction _zombiealpha) (`Timeline|Zombify` :!via `PlayFromStart`)
    (:`Update`
      (`MaterialInstanceDynamic.SetScalarParameterValue` (`self.MaterialInstance`) "bZombie?" (`KismetMathLibrary.Lerp` 0.0 1.0 _zombiealpha)))
    (:`Finished`
      (`KismetSystemLibrary.Delay` 1.0)
      (bind _returnvalue_2 (`|SpawnActorFromClass` "/Game/Blueprints/Controllers/AIC_EnemyController.AIC_EnemyController_C" (`KismetMathLibrary.MakeTransform` (0.0 0.0 0.0)) "Undefined" "MultiplyWithRoot" null null))
      (`Controller.Possess` _returnvalue_2 self)
      (`CharacterMovementComponent.SetMovementMode` (`self.CharacterMovement`) "MOVE_Walking" 0)
      (`SkeletalMeshComponent.SetAnimInstanceClass` (`self.Mesh`) "/Game/Blueprints/Animations/ABP_EnemyZombie.ABP_EnemyZombie_C")
      (`self.EnableInput` _playerref_2 (`GameplayStatics.GetPlayerController` 0))
      (`UserWidget.AddToViewport` (`/Game/Blueprints/Characters/BP_Character.Hud` _playerref_2) 0))))

(fn `UserConstructionScript`
  (`parent.UserConstructionScript`))