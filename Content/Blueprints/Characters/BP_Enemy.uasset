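; Enemy character, with a zombie death animation, that takes typed damage and attacks the player.
; Damage subtracts a value looked up by type in the game mode's table; at zero health it records its death in LevelState, drops its controller and plays the death montage.
; Capsule overlaps report player attack range to AIC_EnemyController.
; AttackCollider starts without collision and sends damage to the player on overlap.
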(event `self.ReceiveBeginPlay`
  (bind _asbp_third_person_game_mode (cast `/Game/ThirdPerson/Blueprints/BP_ThirdPersonGameMode` (`GameplayStatics.GetGameMode`)))
  (set `self.DamageValues` (`/Game/ThirdPerson/Blueprints/BP_ThirdPersonGameMode.DamageValues` _asbp_third_person_game_mode))
  (`PrimitiveComponent.SetCollisionEnabled` (`self.AttackCollider`) "NoCollision"))

(event `/Game/Blueprints/Interfaces/BPI_Damage.Damage`
  (params (Type :type String))
  (if (`self.bAlive`)
    (set `self.Health` (- (`self.Health`) (`BlueprintMapLibrary.Map_Find` (`self.DamageValues`) Type)))
    (if (<= (`self.Health`) 0)
      (bind _output_get (set `self.bAlive` false))
      (`BlueprintMapLibrary.Map_Add` (`/Game/Blueprints/Data/BP_LevelState.Spawn?` (`self.LevelState`)) (`self.Id`) _output_get)
      ; Reemplazar por comportamiento
      (`self.DetachFromControllerPendingDestroy`)
      (`CharacterMovementComponent.DisableMovement` (`self.CharacterMovement`))
      (`|PlayMontage` (`self.Mesh`) "/Game/Animations/AM_ZombieDeath1.AM_ZombieDeath1"
        (:`then`
          (`PrimitiveComponent.SetCollisionEnabled` (`self.CapsuleComponent`) "NoCollision")
          (`KismetSystemLibrary.PrintString` "Enemy Killed")))
      (else
        (`KismetSystemLibrary.PrintString` (`KismetStringLibrary.Concat_StrStr` (`KismetStringLibrary.Conv_IntToString` (`self.Health`)) "HP Left"))))))

(event `self.CapsuleComponent.OnComponentBeginOverlap`
  (params (OverlappedComponent :type "PrimitiveComponent Object Reference") (OtherActor :type "Actor Object Reference") (OtherComp :type "PrimitiveComponent Object Reference") (OtherBodyIndex :type Integer) (bFromSweep :type Boolean) (SweepResult :type "HitResult Structure (by ref)"))
  (if (`self.ActorHasTag` OtherActor "Player")
    (bind _output_get (set `self.AttackRange` true))
    (bind _asaic_enemy_controller (cast `/Game/Blueprints/Controllers/AIC_EnemyController` (`self.GetController`)))
    (`/Engine/EditorBlueprintResources/StandardMacros.IsValid` _asaic_enemy_controller
      (:`Is Valid`
        (`/Game/Blueprints/Controllers/AIC_EnemyController.AttackRange` _asaic_enemy_controller _output_get)))))

(event `self.CapsuleComponent.OnComponentEndOverlap`
  (params (OverlappedComponent :type "PrimitiveComponent Object Reference") (OtherActor :type "Actor Object Reference") (OtherComp :type "PrimitiveComponent Object Reference") (OtherBodyIndex :type Integer))
  (if (`self.ActorHasTag` OtherActor "Player")
    (bind _output_get (set `self.AttackRange` false))
    (bind _asaic_enemy_controller (cast `/Game/Blueprints/Controllers/AIC_EnemyController` (`self.GetController`)))
    (`/Engine/EditorBlueprintResources/StandardMacros.IsValid` _asaic_enemy_controller
      (:`Is Valid`
        (`/Game/Blueprints/Controllers/AIC_EnemyController.AttackRange` _asaic_enemy_controller _output_get)))))

(event `self.AttackCollider.OnComponentBeginOverlap`
  (params (OverlappedComponent :type "PrimitiveComponent Object Reference") (OtherActor :type "Actor Object Reference") (OtherComp :type "PrimitiveComponent Object Reference") (OtherBodyIndex :type Integer) (bFromSweep :type Boolean) (SweepResult :type "HitResult Structure (by ref)"))
  (if (`self.ActorHasTag` OtherActor "Player")
    (message `/Game/Blueprints/Interfaces/BPI_Damage.Damage` OtherActor "Enemy")))

(fn `UserConstructionScript`)